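; GM_GameMode is a game mode that sets up the player's flying pawn at level start.
; On BeginPlay it waits briefly, finds and caches the BP_FRIWorldGenerator actor, then spawns a BP_FlyingPawn at the PlayerStart.
; It possesses the pawn with the first player controller and passes it the world generator reference.
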(event `self.ReceiveBeginPlay`
  (`KismetSystemLibrary.Delay` 0.2)
  (bind _returnvalue (`GameplayStatics.GetActorOfClass` "/Game/Blueprints/BP_FRIWorldGenerator.BP_FRIWorldGenerator_C"))
  (set `self.WorldGenerator` _returnvalue)
  (bind _returnvalue_2 (`|SpawnActorFromClass` "/Game/Blueprints/BP_FlyingPawn.BP_FlyingPawn_C" (`self.GetTransform` (`self.K2_FindPlayerStart` null)) "Undefined" "MultiplyWithRoot" null null))
  (bind _output_get (set `self.FlyingPawn` _returnvalue_2))
  (`Controller.Possess` (`GameplayStatics.GetPlayerController` 0) _output_get)
  (set `/Game/Blueprints/BP_FlyingPawn.worldGeneratorRef` (`self.WorldGenerator`) (`self.FlyingPawn`)))

(fn `UserConstructionScript`)
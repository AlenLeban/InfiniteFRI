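; Tile generator actor Blueprint that shows generation status through a progress widget component.
; On BeginPlay it casts the component's widget to W_GeneratorProgress, passes itself as GeneratorRef and caches the widget.
; When generation finishes, it hides the widget, first showing a failure message for a short delay if retries reached the maximum.
; UpdateProgressVisual is empty, and no generation logic appears in these graphs.
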(event `self.ReceiveBeginPlay`
  (bind _asw_generator_progress (cast `/Game/Blueprints/W_GeneratorProgress` (`WidgetComponent.GetUserWidgetObject` (`self.ProgressWidget`))))
  (set `/Game/Blueprints/W_GeneratorProgress.generatorRef` self _asw_generator_progress)
  (set `self.W_Progress` _asw_generator_progress))

(event `self.UpdateProgressVisual`)

(event `self.OnGeneratorFinished`
  (if (== (`self.retries`) (`self.maxRetries`))
    (set `/Game/Blueprints/W_GeneratorProgress.errorMessage` "Failed" (`self.W_Progress`))
    (`KismetSystemLibrary.Delay` 2.0))
  (`SceneComponent.SetVisibility` (`self.ProgressWidget`) false false))

(fn `UserConstructionScript`)